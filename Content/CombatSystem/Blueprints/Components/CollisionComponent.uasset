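; A combat collision component that detects hits along a mesh between two sockets while collision is enabled.
; Each tick it runs a multi-sphere object trace from start to end socket of the assigned mesh, skipping ignored actors.
; Each actor is reported through an OnHit call only once per activation, as enabling collision clears the already-hit list.
; Functions expose hit state and manage the ignore list.
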(event Custom|DisableCollision
  ;[1 0 0] Disable Collision
  (Variables|Default|SetbIsCollisionEnabled? false))

(event Custom|EnableCollision
  ;[1 0 0] Enable Collision
  (CallFunction|ClearHitActors)
  (Variables|Default|SetbIsCollisionEnabled? true))

(event Custom|ClearHitActors
  ;[1 0 0] Clear Hit Actors
  (Utilities|Array|Clear (Variables|Default|GetAlreadyHitActors)))

(event Custom|CollisionTrace
  (bind _collisionmeshcomponent (Variables|Default|GetCollisionMeshComponent))
  ;[1 0 0] Collsion Trace
  (bind _outhits (Collision|MultiSphereTraceForObjects (Transformation|GetSocketLocation _collisionmeshcomponent (Variables|Initialization|GetStartSocketName)) (Transformation|GetSocketLocation _collisionmeshcomponent (Variables|Initialization|GetEndSocketName)) (Variables|Initialization|GetTraceRadius) (Variables|Initialization|GetCollisionObjectTypes) false (Variables|Default|GetActorsToIgnore) (Variables|Initialization|GetDrawDebugType)))
  (for _array_element _outhits
    (bind _output_get (Variables|Default|SetLastHit _array_element))
    (if (not (Utilities|Array|ContainsItem (Variables|Default|GetAlreadyHitActors) (.HitActor (Collision|BreakHitResult _output_get))))
      (bind _output_get_2 (Variables|Default|SetHit%20Actor (.HitActor (Collision|BreakHitResult _output_get))))
      (Utilities|Array|Add (Variables|Default|GetAlreadyHitActors) _output_get_2)
      (Default|CallOnHit (Variables|Default|GetLastHit)))))

(event Custom|SetCollisionMesh
  (params (MeshComponent :type Primitive%20Component%20Object%20Reference))
  ;[1 0 0] Set Collision Mesh Component
  (Variables|Default|SetCollisionMeshComponent MeshComponent))

(event EventTick
  (params (DeltaSeconds :type Float%20%28single-precision%29))
  (if (Variables|Default|GetbIsCollisionEnabled?)
    (CallFunction|CollisionTrace)))

(fn GetAlreadyHitActors
  (return (Variables|Default|GetAlreadyHitActors)))

(fn IsCollisonEnabled?
  (return (Variables|Default|GetbIsCollisionEnabled?)))

(fn GetLastHit
  (return (Variables|Default|GetLastHit)))

(fn GetCollisionMeshComponent
  (return (Variables|Default|GetCollisionMeshComponent)))

(fn AddActortoIgnore
  (params (AddToIgnore :type Actor%20Object%20Reference%20%28by%20ref%29))
  (Utilities|Array|AddUnique (Variables|Default|GetActorsToIgnore) AddToIgnore))

(fn RemoveActorfromIgnore
  (params (AddToIgnore :type Actor%20Object%20Reference%20%28by%20ref%29))
  (Utilities|Array|RemoveItem (Variables|Default|GetActorsToIgnore) AddToIgnore))

(fn GetActorstoIgnore
  (return (Variables|Default|GetActorsToIgnore)))