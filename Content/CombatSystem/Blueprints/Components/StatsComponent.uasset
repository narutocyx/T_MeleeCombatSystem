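; Combat system component that stores an actor's stats and handles incoming damage.
; InitializeStats seeds the CurrentStats map from BaseStats, whose structs hold a base and max value per stat enum.
; ModifyCurrentStatValue clamps changes between zero and max, while direct sets are unclamped.
; TakeDamage lowers one stat (presumably health) and, at zero, switches the owner's StateManagerComponent state, likely to death.
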(event EventBeginPlay)

(event EventTick
  (params (DeltaSeconds :type Float%20%28single-precision%29)))

(fn InitializeStats
  (bind _keys (Utilities|Map|Keys (Variables|BaseStats|GetBaseStats)))
  (for _array_element _keys
    (CallFunction|SetCurrentStatValue _array_element (.basevalue (.Value (Utilities|Map|Find (Variables|BaseStats|GetBaseStats) _array_element))))))

(fn SetCurrentStatValue
  (params (Stat :type E_Stats%20Enum%20%28by%20ref%29 :default "NewEnumerator0") (Value :type Float%20%28double-precision%29%20%28by%20ref%29))
  (Utilities|Map|Add (Variables|Default|GetCurrentStats) Stat Value))

(fn GetCurrentStatValue
  (params (Stat :type E_Stats%20Enum :default "NewEnumerator0"))
  (return (.Value (Utilities|Map|Find (Variables|Default|GetCurrentStats) Stat))))

(fn ModifyCurrentStatValue
  (params (Stat :type E_Stats%20Enum :default "NewEnumerator0") (Value :type Float%20%28double-precision%29))
  (if (!= Value 0.0)
    (LocalVariables|SetL_Value 0.0)
    (CallFunction|SetCurrentStatValue Stat (Math|Float|Clamp(Float) (+ Value (CallFunction|GetCurrentStatValue Stat)) 0.0 (BaseStats|GetMaxStatValue Stat)))))

(fn SetBaseStatValue
  (params (Stat :type E_Stats%20Enum :default "NewEnumerator0") (Value :type Float%20%28double-precision%29))
  (bind _structout (Utilities|Struct|SetmembersinS_BaseStat (.Value (Utilities|Map|Find (Variables|BaseStats|GetBaseStats) Stat)) Value))
  (Utilities|Map|Add (Variables|BaseStats|GetBaseStats) Stat _structout))

(fn SetMaxStatValue
  (params (Stat :type E_Stats%20Enum :default "NewEnumerator0") (Value :type Float%20%28double-precision%29))
  (bind _structout (Utilities|Struct|SetmembersinS_BaseStat (.Value (Utilities|Map|Find (Variables|BaseStats|GetBaseStats) Stat)) Value))
  (Utilities|Map|Add (Variables|BaseStats|GetBaseStats) Stat _structout))

(fn GetBaseStatValue
  (params (Stat :type E_Stats%20Enum :default "NewEnumerator0"))
  (return (.basevalue (.Value (Utilities|Map|Find (Variables|BaseStats|GetBaseStats) Stat)))))

(fn GetMaxStatValue
  (params (Stat :type E_Stats%20Enum :default "NewEnumerator0"))
  (return (.maxvalue (.Value (Utilities|Map|Find (Variables|BaseStats|GetBaseStats) Stat)))))

(fn TakeDamage
  (params (InDamage :type Float%20%28double-precision%29))
  (CallFunction|ModifyCurrentStatValue "NewEnumerator1" (* InDamage -1.0))
  (if (<= (CallFunction|GetCurrentStatValue "NewEnumerator1") 0.0)
    (Default|SetState (Actor|GetComponentbyClass (Components|GetOwner) "/Game/CombatSystem/Blueprints/Components/StateManagerComponent.StateManagerComponent_C") "NewEnumerator4")))