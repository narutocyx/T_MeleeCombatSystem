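; Base actor for equippable items in the combat system, tracking whether the item is equipped.
; Equipping sets the flag and snaps the item to the owning Character's mesh at AttachSocketName, while unequipping only clears the flag.
; GetItemMesh returns the static mesh component if it has a mesh, otherwise the skeletal one, and prints an error if neither does.
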(event EventBeginPlay)

(event Collision|EventActorBeginOverlap
  (params (OtherActor :type Actor%20Object%20Reference)))

(event EventTick
  (params (DeltaSeconds :type Float%20%28single-precision%29)))

(fn ConstructionScript)

(fn GetItemMesh
  (Utilities|IsValid (Variables|/Script/Engine.StaticMeshComponent|GetStaticMesh (Variables|Default|GetItemStaticMesh))
    (:Is%20Valid
      (return (Variables|Default|GetItemStaticMesh)))
    (:Is%20Not%20Valid
      (Utilities|IsValid (Variables|/Script/Engine.SkeletalMeshComponent|GetSkeletalMeshAsset (Variables|Default|GetItemSkeletalMesh))
        (:Is%20Valid
          (return (Variables|Default|GetItemSkeletalMesh)))
        (:Is%20Not%20Valid
          (Development|PrintString "Error!!!"))))))

(fn OnEquipped
  (Variables|Default|SetbIsEquipped? true)
  (ItemMesh|AttachActor (Variables|Default|GetAttachSocketName)))

(fn OnUnequipped
  (Variables|Default|SetbIsEquipped? false))

(fn AttachActor
  (params (SocketName :type Name))
  (Transformation|AttachComponentToComponent (Variables|/Script/Engine.Character|GetMesh (.AsCharacter (Utilities|Casting|CastToCharacter (Components|GetOwner)))) SocketName "SnapToTarget" "SnapToTarget" "SnapToTarget" true))

(fn SetIsEqiupped
  (params (bIsEquipped? :type Boolean))
  (Variables|Default|SetbIsEquipped? bIsEquipped?))

(fn IsEquipped?
  (return (Variables|Default|GetbIsEquipped?)))